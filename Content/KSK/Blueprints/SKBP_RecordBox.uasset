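; Trigger box actor that records captured audio while a top-down character stands inside, producing a meeting recording for speech-to-text.
; Overlap events show or hide the player widget's looping recording indicator.
; Tick polls occupancy through DoOnce gates, starting audio capture and master submix recording, then stopping when the box empties.
; It exports a WAV to the project's Sound folder and, after a short delay, passes its path to SKBP_AudioActor's ReqSoundToText.
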(event OnComponentBeginOverlap(Box)
  (params (OverlappedComponent :type Primitive%20Component%20Object%20Reference) (OtherActor :type Actor%20Object%20Reference) (OtherComp :type Primitive%20Component%20Object%20Reference) (OtherBodyIndex :type Integer) (bFromSweep :type Boolean) (SweepResult :type Hit%20Result%20Structure%20%28by%20ref%29))
  (for _array_element (Collision|GetOverlappingActors "/Game/KHH/Blueprints/BP_TopDownCharacter1.BP_TopDownCharacter1_C" :!class /Script/Engine.Actor)
    (bind _asbp_top_down_character_1 (Utilities|Casting|CastToBP_TopDownCharacter1 _array_element))
    (Widget|SetVisibility (Variables|/Game/KHH/UI/UI/WBP_Player.WBP_Player_C|GetRecordingText (Variables|/Game/KHH/Blueprints/BP_TopDownCharacter1.BP_TopDownCharacter1_C|GetAs%20WBP%20Player _asbp_top_down_character_1)) "Visible")
    (UserInterface|Animation|PlayAnimation (Variables|/Game/KHH/Blueprints/BP_TopDownCharacter1.BP_TopDownCharacter1_C|GetAs%20WBP%20Player _asbp_top_down_character_1) (Variables|/Game/KHH/UI/UI/WBP_Player.WBP_Player_C|GetRecording (Variables|/Game/KHH/Blueprints/BP_TopDownCharacter1.BP_TopDownCharacter1_C|GetAs%20WBP%20Player _asbp_top_down_character_1)) 0.0 0 "Forward" 1.0 false)))

(event OnComponentEndOverlap(Box)
  (params (OverlappedComponent :type Primitive%20Component%20Object%20Reference) (OtherActor :type Actor%20Object%20Reference) (OtherComp :type Primitive%20Component%20Object%20Reference) (OtherBodyIndex :type Integer))
  (bind _asbp_top_down_character_1 (Utilities|Casting|CastToBP_TopDownCharacter1 OtherActor))
  (Widget|SetVisibility (Variables|/Game/KHH/UI/UI/WBP_Player.WBP_Player_C|GetRecordingText (Variables|/Game/KHH/Blueprints/BP_TopDownCharacter1.BP_TopDownCharacter1_C|GetAs%20WBP%20Player _asbp_top_down_character_1)) "Hidden")
  (Class|UserWidget|StopAnimation (Variables|/Game/KHH/Blueprints/BP_TopDownCharacter1.BP_TopDownCharacter1_C|GetAs%20WBP%20Player _asbp_top_down_character_1) (Variables|/Game/KHH/UI/UI/WBP_Player.WBP_Player_C|GetRecording (Variables|/Game/KHH/Blueprints/BP_TopDownCharacter1.BP_TopDownCharacter1_C|GetAs%20WBP%20Player _asbp_top_down_character_1))))

(event EventTick
  (params (DeltaSeconds :type Float%20%28single-precision%29))
  (bind _returnvalue (Class|KismetSystemLibrary|GetProjectContentDirectory))
  (bind _returnvalue_2 (Utilities|String|Append _returnvalue "Sound/"))
  (if (> (Utilities|Array|Length (Collision|GetOverlappingActors "/Game/KHH/Blueprints/BP_TopDownCharacter1.BP_TopDownCharacter1_C" :!class /Script/Engine.Actor)) 0)
    (Utilities|FlowControl|DoOnce false :!label _label
      (:Completed
        (CameraShake|Start (Variables|Default|GetAudioCapture))
        (Class|AudioMixerBlueprintLibrary|StartRecordingOutput 0.0 "/Engine/EngineSounds/Submixes/MasterSubmixDefault.MasterSubmixDefault")
        (Variables|Default|SetbRecording true)
        (Development|PrintString "StartRecord")))
    (else
      (Utilities|FlowControl|DoOnce false :!label _label_2
        (:Completed
          (if (Variables|Default|GetbRecording)
            (Audio|Components|Audio|Stop (Variables|Default|GetAudioCapture))
            (Development|PrintString _returnvalue_2)
            (Class|AudioMixerBlueprintLibrary|StopRecordingOutput "WavFile" "MeetingContext" _returnvalue_2 "/Engine/EngineSounds/Submixes/MasterSubmixDefault.MasterSubmixDefault" 0)
            (Variables|Default|SetbRecording false)
            (Utilities|FlowControl|Delay 1.0)
            (bind _returnvalue_3 (Actor|GetActorOfClass "/Game/KSK/Blueprints/SKBP_AudioActor.SKBP_AudioActor_C"))
            (Class|HttpLib|ReqSoundtoText _returnvalue_3 (Utilities|String|Append _returnvalue_2 "MeetingContext.wav"))
            (Development|PrintString "EndRecord"))
          (Utilities|FlowControl|Sequence
            (:then_0
              (goto _label Reset))
            (:then_1
              (goto _label_2 Reset))))))))

(fn ConstructionScript)