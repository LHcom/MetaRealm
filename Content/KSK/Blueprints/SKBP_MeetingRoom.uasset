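; Meeting room actor that records audio while any BP_TopDownCharacter overlaps it.
; Tick polls overlaps and, through a DoOnce gate, starts AudioCapture and master submix recording.
; When the last character leaves, it stops both, exports a MeetingContext WAV to the project content Sound folder and re-arms the gate.
; Box overlap and click events only print debug strings.
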(event OnComponentBeginOverlap(Box)
  (params (OverlappedComponent :type Primitive%20Component%20Object%20Reference) (OtherActor :type Actor%20Object%20Reference) (OtherComp :type Primitive%20Component%20Object%20Reference) (OtherBodyIndex :type Integer) (bFromSweep :type Boolean) (SweepResult :type Hit%20Result%20Structure%20%28by%20ref%29))
  (bind _asbp_top_down_character (Utilities|Casting|CastToBP_TopDownCharacter OtherActor))
  (Development|PrintString (Utilities|GetDisplayName _asbp_top_down_character)))

(event OnClicked(Box)
  (params (TouchedComponent :type Primitive%20Component%20Object%20Reference) (ButtonPressed :type Key%20Structure :default "None"))
  (Development|PrintString "Hello"))

(event EventTick
  (params (DeltaSeconds :type Float%20%28single-precision%29))
  (bind _returnvalue (Class|KismetSystemLibrary|GetProjectContentDirectory))
  (if (> (Utilities|Array|Length (Collision|GetOverlappingActors "/Game/TopDown/Blueprints/BP_TopDownCharacter.BP_TopDownCharacter_C" :!class /Script/Engine.Actor)) 0)
    (Utilities|FlowControl|DoOnce false :!label _label
      (:Completed
        (CameraShake|Start (Variables|Default|GetAudioCapture))
        (Class|AudioMixerBlueprintLibrary|StartRecordingOutput 0.0 "/Engine/EngineSounds/Submixes/MasterSubmixDefault.MasterSubmixDefault")
        (Variables|Default|SetbRecording true)))
    (elif (Variables|Default|GetbRecording)
      (Audio|Components|Audio|Stop (Variables|Default|GetAudioCapture))
      (Development|PrintString _returnvalue)
      (Class|AudioMixerBlueprintLibrary|StopRecordingOutput "WavFile" "MeetingContext" (Utilities|String|Append _returnvalue "/Sound") "/Engine/EngineSounds/Submixes/MasterSubmixDefault.MasterSubmixDefault" 0)
      (Variables|Default|SetbRecording false)
      (goto _label Reset))))

(fn ConstructionScript)