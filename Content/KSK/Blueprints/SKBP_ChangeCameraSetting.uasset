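; A trigger volume Blueprint that changes the top-down character's camera framing while the character is inside its Box.
; On begin overlap it caches the BP_TopDownCharacter and its SpringArm, then shortens the arm and raises its relative location.
; When that cached character leaves, it lengthens the arm and lowers it to fixed values rather than saved originals.
; Both changes apply instantly and set the same world rotation.
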(event OnComponentBeginOverlap(Box)
  (params (OverlappedComponent :type Primitive%20Component%20Object%20Reference) (OtherActor :type Actor%20Object%20Reference) (OtherComp :type Primitive%20Component%20Object%20Reference) (OtherBodyIndex :type Integer) (bFromSweep :type Boolean) (SweepResult :type Hit%20Result%20Structure%20%28by%20ref%29))
  (bind _asbp_top_down_character_1 (Utilities|Casting|CastToBP_TopDownCharacter1 OtherActor))
  (bind _output_get (Variables|Default|SetAs%20BP%20Top%20Down%20Character%201 _asbp_top_down_character_1))
  (bind _output_get_2 (Variables|Default|SetSpring%20Arm_0 (Variables|/Game/KHH/Blueprints/BP_TopDownCharacter1.BP_TopDownCharacter1_C|GetSpringArm _output_get)))
  (Variables|/Script/Engine.SpringArmComponent|SetTargetArmLength _output_get_2 2e+03)
  (Transformation|SetWorldRotation (Variables|Default|GetSpring%20Arm_0) "-43.000000,0.000000,0.000000" false false)
  (Transformation|SetRelativeLocation (Variables|Default|GetSpring%20Arm_0) "0.000000,0.000000,150.000000" false false))

(event OnComponentEndOverlap(Box)
  (params (OverlappedComponent :type Primitive%20Component%20Object%20Reference) (OtherActor :type Actor%20Object%20Reference) (OtherComp :type Primitive%20Component%20Object%20Reference) (OtherBodyIndex :type Integer))
  (if (== OtherActor (Variables|Default|GetAs%20BP%20Top%20Down%20Character%201))
    (Variables|/Script/Engine.SpringArmComponent|SetTargetArmLength (Variables|Default|GetSpring%20Arm_0) 3.5e+03)
    (Transformation|SetWorldRotation (Variables|Default|GetSpring%20Arm_0) "-43.000000,0.000000,0.000000" false false)
    (Transformation|SetRelativeLocation (Variables|Default|GetSpring%20Arm_0) "0.000000,0.000000,-150.000000" false false)))

(fn ConstructionScript)