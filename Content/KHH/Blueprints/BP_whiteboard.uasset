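; BP_whiteboard is a whiteboard actor that shows an interaction prompt while the player's top-down character is inside its trigger box.
; On BeginPlay it caches player 0's BP_TopDownCharacter, then creates a WBP_Interaction widget and adds it to the viewport hidden.
; Box begin and end overlap events toggle the widget's visibility, responding only to that cached character.
; It contains no input handling or further interaction logic.
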(event OnComponentBeginOverlap(Box)
  (params (OverlappedComponent :type Primitive%20Component%20Object%20Reference) (OtherActor :type Actor%20Object%20Reference) (OtherComp :type Primitive%20Component%20Object%20Reference) (OtherBodyIndex :type Integer) (bFromSweep :type Boolean) (SweepResult :type Hit%20Result%20Structure%20%28by%20ref%29))
  (if (== (Variables|Default|GetAs%20BP%20Top%20Down%20Character) OtherActor)
    (Widget|SetVisibility (Variables|Default|GetNewVar) "Visible")))

(event OnComponentEndOverlap(Box)
  (params (OverlappedComponent :type Primitive%20Component%20Object%20Reference) (OtherActor :type Actor%20Object%20Reference) (OtherComp :type Primitive%20Component%20Object%20Reference) (OtherBodyIndex :type Integer))
  (if (== (Variables|Default|GetAs%20BP%20Top%20Down%20Character) OtherActor)
    (Widget|SetVisibility (Variables|Default|GetNewVar) "Hidden")))

(event EventBeginPlay
  (bind _asbp_top_down_character (Utilities|Casting|CastToBP_TopDownCharacter (Game|GetPlayerCharacter 0)))
  (Variables|Default|SetAs%20BP%20Top%20Down%20Character _asbp_top_down_character)
  (bind _returnvalue (UserInterface|CreateWidget "/Game/KHH/UI/UI/WBP_Interaction.WBP_Interaction_C"))
  (bind _output_get (Variables|Default|SetNewVar _returnvalue))
  (UserInterface|Viewport|AddtoViewport _output_get 0)
  (Widget|SetVisibility _output_get "Hidden"))

(event Collision|EventActorBeginOverlap
  (params (OtherActor :type Actor%20Object%20Reference)))

(event EventTick
  (params (DeltaSeconds :type Float%20%28single-precision%29)))

(fn ConstructionScript)